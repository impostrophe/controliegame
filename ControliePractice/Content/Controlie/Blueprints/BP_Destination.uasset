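; BP_Destination is a destination actor that AI characters use to replenish their stats.
; UseItem adds each stat's own StatRestore from the character's AIStatArray, clamped to its min and max, skipping index 0.
; A negative StatRestore at index 0 is instead applied as damage to the character.
; GetStateIndex returns 0, and the logic for registering destination locations is unconnected.
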(event EventBeginPlay
  ;[1 0.4536 0] need base destination array maybe
)

(event EventUseItem
  (params (AI_Character :type AIS%20Character%20Object%20Reference))
  (bind _aistatarray (Variables|/Game/Controlie/AIS/AIS_Character.AIS_Character_C|GetAIStatArray AI_Character))
  (bind _output (Utilities|Array|Get(acopy) _aistatarray))
  (for _index (range 1 (Utilities|Array|LastIndex _aistatarray))
    (Utilities|Array|SetArrayElem _aistatarray _index (Utilities|Struct|MakeStatStruct (Math|Float|Clamp(Float) (+ (.currentstatvalue (Utilities|Array|Get(acopy) _aistatarray _index)) (.statrestore (Utilities|Array|Get(acopy) _aistatarray _index))) (.statmin (Utilities|Array|Get(acopy) _aistatarray _index)) (.statmax (Utilities|Array|Get(acopy) _aistatarray _index))) (.statmin (Utilities|Array|Get(acopy) _aistatarray _index)) (.statmax (Utilities|Array|Get(acopy) _aistatarray _index)) (.statdesirability (Utilities|Array|Get(acopy) _aistatarray _index)) (.statdecayrate (Utilities|Array|Get(acopy) _aistatarray _index)) (.statrestore (Utilities|Array|Get(acopy) _aistatarray _index)) (.statbehaviors (Utilities|Array|Get(acopy) _aistatarray _index)) (.useitemsound (Utilities|Array|Get(acopy) _aistatarray _index)))))
  (if (< (.statrestore _output) 0.0)
    (Game|Damage|ApplyDamage AI_Character (Math|Float|Absolute(Float) (.statrestore _output)) 0 self)))

(fn ConstructionScript)

(fn GetStateIndex
  (return 0))