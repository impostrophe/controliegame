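; Fun destination Blueprint for a mountain climb, which an AI character performs when DoAction is called on it.
; BeginPlay gathers seven climb point components into an ordered array.
; DoAction marks the character busy, stores its starting location, then teleports it through the points at one-second intervals before clearing busy status.
; The starting location goes unused and the array counter is never reset in this graph.
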(event EventBeginPlay
  (|CallParentFunction)
  (Variables|Default|SetClimbPoints (Utilities|Array|MakeArray (Variables|Default|GetClimbPoint0) (Variables|Default|GetClimbPoint1) (Variables|Default|GetClimbPoint2) (Variables|Default|GetClimbPoint3) (Variables|Default|GetClimbPoint4) (Variables|Default|GetClimbPoint5) (Variables|Default|GetClimbPoint6))))

(event EventDoAction
  (params (AI_Character :type AIS%20Character%20Object%20Reference))
  (bind _climbpoints (Variables|Default|GetClimbPoints))
  (CallFunction|SetBusyStatus AI_Character true)
  (Variables|Default|SetStartingpoint (Transformation|GetActorLocation AI_Character))
  (if (== (Variables|Default|GetArrayCounter) (Utilities|Array|Length _climbpoints)) :!label _label
    (CallFunction|SetBusyStatus AI_Character false)
    (else
      (Transformation|Teleport AI_Character (Transformation|GetWorldLocation (Utilities|Array|Get(acopy) _climbpoints (Variables|Default|GetArrayCounter))) "0, 0, 0")
      (Utilities|FlowControl|Delay 1.0)
      (Math|Integer|IncrementInt (Variables|Default|GetArrayCounter)
        (:%20%20
          (goto _label))))))

(fn ConstructionScript
  (|CallParentFunction))