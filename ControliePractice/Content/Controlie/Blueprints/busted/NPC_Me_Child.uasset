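; NPC_Me_Child is a child NPC Blueprint that wanders between destinations held by ControlieGameState.
; After a startup delay, a looping timer runs SelectAction, which, if TimeToMove is set, sends it via AIMoveTo to a random destination's Box.
; An ActionInProgress flag and DoOnce gate moves, resetting only when a move succeeds.
; PawnSensing prints a debug string and applies large upward movement input to the seen pawn; InteractionRadius overlap is empty.
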(event OnSeePawn(PawnSensing)
  (params (Pawn :type Pawn%20Object%20Reference))
  (Development|PrintString "sweet!")
  (Pawn|Input|AddMovementInput Pawn "0, 0,50000.000000" 1.0 false))

(event OnComponentBeginOverlap(InteractionRadius)
  (params (OverlappedComponent :type Primitive%20Component%20Object%20Reference) (OtherActor :type Actor%20Object%20Reference) (OtherComp :type Primitive%20Component%20Object%20Reference) (OtherBodyIndex :type Integer) (bFromSweep :type Boolean) (SweepResult :type Hit%20Result%20Structure%20%28by%20ref%29)))

(event Custom|SelectAction
  (bind _gamestate_0 (Variables|Default|GetGameState_0))
  (bind _destinations (Variables|/Game/Controlie/Game/ControlieGameState.ControlieGameState_C|GetDestinations _gamestate_0))
  (if (not (Variables|Default|GetActionInProgress))
    (Variables|Default|SetActionInProgress true)
    (bind _ascontrolie_game_state (Utilities|Casting|CastToControlieGameState (Game|GetGameState)))
    (if (Variables|/Game/Controlie/Game/ControlieGameState.ControlieGameState_C|GettimeToMove _ascontrolie_game_state)
      (Utilities|FlowControl|DoOnce false :!label _label
        (:Completed
          (AI|AIMoveTo self (Transformation|GetWorldLocation (Variables|/Game/Controlie/Blueprints/BP_Destination.BP_Destination_C|GetBox (Utilities|Array|Get(acopy) _destinations (Math|Random|RandomIntegerinRange 0 (Utilities|Array|Length _destinations))))) 0 5.0 false
            (:OnSuccess
              (Variables|Default|SetActionInProgress false)
              (goto _label Reset))))))))

(event EventBeginPlay
  (Utilities|FlowControl|Delay 5.0)
  (Utilities|Time|SetTimerbyEvent (delegate Custom|SelectAction) 5.0 true)
  (bind _ascontrolie_game_state (Utilities|Casting|CastToControlieGameState (Game|GetGameState)))
  (Variables|Default|SetGameState_0 _ascontrolie_game_state))

(event Collision|EventActorBeginOverlap
  (params (OtherActor :type Actor%20Object%20Reference))
  (|CallParentFunction OtherActor) ; This node is disabled and will not be called.\nDrag off pins to build functionality.
)

(event EventTick
  (params (DeltaSeconds :type Float%20%28single-precision%29))
  (|CallParentFunction DeltaSeconds) ; This node is disabled and will not be called.\nDrag off pins to build functionality.
)

(fn ConstructionScript
  (|CallParentFunction))