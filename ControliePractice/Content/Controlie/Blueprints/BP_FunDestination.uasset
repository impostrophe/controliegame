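; BP_FunDestination is an entertainment destination that AI characters use to change one of their stats.
; On BeginPlay it adds itself to the game state's FunDestNew list and registers as a sight perception stimulus.
; UseItem adds the entertainment restore value for the primary stat index to the character's stat, clamped to its range.
; A negative restore value also deals damage of that magnitude to the character.
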(event EventBeginPlay
  (bind _self self)
  (bind _ascontrolie_game_state (Utilities|Casting|CastToControlieGameState (Game|GetGameState)))
  (Utilities|Array|AddUnique (Variables|/Game/Controlie/Game/ControlieGameState.ControlieGameState_C|GetFunDestNew _ascontrolie_game_state) _self)
  (Class|AIPerceptionSystem|RegisterPerceptionStimuliSource "/Script/AIModule.AISense_Sight" _self))

(event EventUseItem
  (params (AI_Character :type AIS%20Character%20Object%20Reference))
  (bind _statrestore_entertainment (Variables|Default|GetStatRestore_Entertainment))
  (bind _aistatarray (Variables|/Game/Controlie/AIS/AIS_Character.AIS_Character_C|GetAIStatArray AI_Character))
  (bind _primarystatindex (Variables|Default|GetPrimaryStatIndex))
  (bind _output (Utilities|Array|Get(acopy) _aistatarray _primarystatindex))
  (bind _output_2 (Utilities|Array|Get(acopy) _statrestore_entertainment _primarystatindex))
  (Utilities|Array|SetArrayElem _aistatarray _primarystatindex (Utilities|Struct|MakeStatStruct (Math|Float|Clamp(Float) (+ (.currentstatvalue _output) (Utilities|Array|Get(acopy) _statrestore_entertainment _primarystatindex)) (.statmin _output) (.statmax _output)) (.statmin _output) (.statmax _output) (.statdesirability _output) (.statdecayrate _output) (.statrestore _output) (.statbehaviors _output)))
  (if (< _output_2 0.0)
    (Game|Damage|ApplyDamage AI_Character (Math|Float|Absolute(Float) _output_2) 0 self)))

(fn ConstructionScript)