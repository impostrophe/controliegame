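; Sleep destination that AI characters use to adjust a stat, presumably as part of a needs system.
; On BeginPlay it adds its mesh location to the game state's SleepDestinations and registers as a sight stimulus for AI perception.
; UseItem adds the StatRestoreAwake value at PrimaryStatIndex to the character's matching stat, clamped to that stat's range.
; A negative restore value also damages the character by the same amount.
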(event EventBeginPlay
  (bind _ascontrolie_game_state (Utilities|Casting|CastToControlieGameState (Game|GetGameState)))
  (Utilities|Array|AddUnique (Variables|/Game/Controlie/Game/ControlieGameState.ControlieGameState_C|GetSleepDestinations _ascontrolie_game_state) (Transformation|GetWorldLocation (Variables|Default|GetStaticMesh)))
  (Class|AIPerceptionSystem|RegisterPerceptionStimuliSource "/Script/AIModule.AISense_Sight"))

(event EventUseItem
  (params (AI_Character :type AIS%20Character%20Object%20Reference))
  (bind _statrestore_awake (Variables|Default|GetStatRestore_Awake))
  (bind _aistatarray (Variables|/Game/Controlie/AIS/AIS_Character.AIS_Character_C|GetAIStatArray AI_Character))
  (bind _primarystatindex (Variables|Default|GetPrimaryStatIndex))
  (bind _output (Utilities|Array|Get(acopy) _aistatarray _primarystatindex))
  (bind _output_2 (Utilities|Array|Get(acopy) _statrestore_awake _primarystatindex))
  (Utilities|Array|SetArrayElem _aistatarray 0 (Utilities|Struct|MakeStatStruct (Math|Float|Clamp(Float) (+ (.currentstatvalue _output) (Utilities|Array|Get(acopy) _statrestore_awake _primarystatindex)) (.statmin _output) (.statmax _output)) (.statmin _output) (.statmax _output) (.statdesirability _output) (.statdecayrate _output) (.statrestore _output) (.statbehaviors _output)))
  (if (< _output_2 0.0)
    (Game|Damage|ApplyDamage AI_Character (Math|Float|Absolute(Float) _output_2) 0 self)))

(fn ConstructionScript)