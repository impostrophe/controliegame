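; BP_StatSpawningActor is a spawner that periodically scatters PlantFoodItem pickups around itself and registers as an AI sight stimulus.
; A looping timer spawns each item above a random navigable point within FarSpawnRange and gives its mesh a random spin.
; Each item receives the spawner's PrimaryStatIndex; a leftover branch that would randomize that index is disconnected and never runs.
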(event Custom|SpawnStatItem
  (bind _returnvalue (Game|SpawnActorfromClass "/Game/Controlie/AIS/BaseClasses/PlantFoodItem.PlantFoodItem_C" (Math|Conversions|ToTransform(Vector) (+ (.RandomLocation (Class|NavigationSystemV1|GetRandomPointinNavigableRadius (Transformation|GetActorLocation) (Variables|Default|GetFarSpawnRange) 0 0)) "0, 0,150.000000")) "AdjustIfPossibleButAlwaysSpawn" 0 (Variables|Default|GetPrimaryStatIndex) 0))
  (Class|PrimitiveComponent|SetPhysicsAngularVelocityinDegrees (Variables|/Game/Controlie/AIS/BaseClasses/GoodFoodClass.GoodFoodClass_C|GetStaticMesh _returnvalue) (* (Math|Random|RandomUnitVector) 1e+02) false "None"))

(event EventBeginPlay
  (Class|AIPerceptionSystem|RegisterPerceptionStimuliSource "/Script/AIModule.AISense_Sight" self)
  (Utilities|Time|SetTimerbyEvent (delegate Custom|SpawnStatItem) (Variables|Default|GetSpawnInterval) true))

(event Collision|EventActorBeginOverlap
  (params (OtherActor :type Actor%20Object%20Reference)))

(event EventTick
  (params (DeltaSeconds :type Float%20%28single-precision%29)))

(fn ConstructionScript)