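; NPC spawn point actor that spawns a configurable class at its Cylinder's location, in either timed or click-triggered mode.
; With SpawnOnTimer set, a looping timer fires at a base rate and adds a random delay before each spawn.
; Otherwise, releasing a click on the Cylinder spawns once, calls PossessAISChar on the player's ControlieCharacter, then destroys the spawn point.
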(event OnReleased(Cylinder)
  (params (TouchedComponent :type Primitive%20Component%20Object%20Reference) (ButtonReleased :type Key%20Structure))
  (if (not (Variables|Default|GetSpawnOnTimer))
    (CallFunction|HandleActorSpawning)))

(event Custom|HandleActorSpawning
  (if (Variables|Default|GetSpawnOnTimer)
    (Utilities|FlowControl|Delay (Math|Random|RandomFloatinRange (Variables|Default|GetSpawnRangeLow) (Variables|Default|GetSpawnRangeHigh))))
  (Game|SpawnActorfromClass (Variables|Default|GetClassToSpawn) (Math|Transform|MakeTransform (.location (Transformation|GetWorldTransform (Variables|Default|GetCylinder))) "0, 0, 0" "1,1,1") "AdjustIfPossibleButAlwaysSpawn" 0 0)
  (if (not (Variables|Default|GetSpawnOnTimer))
    (bind _ascontrolie_character (Utilities|Casting|CastToControlieCharacter (Game|GetPlayerCharacter 0)))
    (Default|PossessAISChar _ascontrolie_character)
    (Actor|DestroyActor)))

(event EventBeginPlay
  (if (Variables|Default|GetSpawnOnTimer)
    (Utilities|Time|SetTimerbyEvent (delegate Custom|HandleActorSpawning) (Variables|Default|GetSpawnBaseRate) true)))

(fn ConstructionScript)